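; Splat capture volume that fills a box with a preview grid of camera positions, rebuilt by the construction script.
; UpdateGrid optionally starts columns at the lowest floor found by repeated line traces, rejects points overlapping StaticMeshActors, and adds the rest as mesh instances.
; GenerateCameraLocations turns each instance into 4, 6 or 12 saved view transforms, per preview mesh selection, with optional random jitter.
; A margin-padded PointCloudBox follows the volume's size.
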(event Custom|UpdateGrid
  (bind _columnhitlocation (Variables|Collision|GetColumnHitLocation))
  (bind _gridspacing (Variables|Grid|GetGridSpacing))
  (bind _volumebox (Variables|Default|GetVolumeBox))
  (bind _gridspacing_2 (Variables|Grid|GetGridSpacing))
  (bind _volumebox_2 (Variables|Default|GetVolumeBox))
  (bind _volumebox_3 (Variables|Default|GetVolumeBox))
  (bind _instancedstaticmesh (Variables|Default|GetInstancedStaticMesh))
  (bind _returnvalue (Components|Box|GetScaledBoxExtent _volumebox_3))
  (bind _returnvalue_2 (Transformation|GetWorldLocation _volumebox))
  (bind _returnvalue_3 (Components|Box|GetScaledBoxExtent _volumebox_2))
  (bind _returnvalue_4 (* (.z _returnvalue) 2.0))
  (bind _returnvalue_5 (* (.x _returnvalue_3) 2.0))
  (bind _returnvalue_6 (* (.y _returnvalue_3) 2.0))
  (bind _returnvalue_7 (/ _returnvalue_4 _gridspacing))
  (bind _returnvalue_8 (/ _returnvalue_5 _gridspacing_2))
  (bind _returnvalue_9 (/ _returnvalue_6 _gridspacing_2))
  (bind _returnvalue_10 (Math|Float|Floor _returnvalue_8))
  (bind _returnvalue_11 (Math|Float|Floor _returnvalue_7))
  (bind _returnvalue_12 (Math|Float|Floor _returnvalue_9))
  ;[1 0.05673 0.7923 1 153] Grid Spawning
  ;;[0.03552 0.5552 1] Setup Instances
  (Components|InstancedStaticMesh|ClearInstances _instancedstaticmesh)
  ;;[0.03552 0.5552 1] Set Static Mesh
  (Components|StaticMesh|SetStaticMesh _instancedstaticmesh (Utilities|Array|Get(acopy) (Variables|PreviewMesh|GetPreviewMesh) (Variables|Grid|GetPreviewMeshSelection)))
  ;;[0.03552 0.5552 1] Clear Transformations
  (Utilities|Array|Clear (Variables|Grid|GetSavedTransforms))
  (Utilities|Array|Clear (Variables|Default|GetSavedInstanceLocations))
  ;;[0.03552 0.5552 1] Resize Point Cloud Box
  (CallFunction|ResizePointCloudBox)
  ;;[0 0.553 1] Calculate Box Top
  (Variables|Grid|SetVolumeBottomZ (- (.z _returnvalue_2) (.z _returnvalue_3)))
  (Variables|Grid|SetVolumeTopZ (+ (.z _returnvalue_2) (.z _returnvalue_3)))
  ;;[0 0.5238 1] X Loop
  (for _index (range 0 (- _returnvalue_10 1))
    ;;[0 0.5238 1] Y Loop
    (for _index_2 (range 0 (- _returnvalue_12 1))
      (if (Variables|Grid|GetbFloorTrace)
        ;;[1 0.5506 0.1137] Floor Trace
        (CallFunction|FloorTrace (.TraceStart (CallFunction|TraceStartEndLocation _index _index_2 (Transformation|GetWorldLocation (Variables|Default|GetVolumeBox)) _returnvalue_10 _returnvalue_12 (Components|Box|GetScaledBoxExtent (Variables|Default|GetVolumeBox)))) (.TraceEnd (CallFunction|TraceStartEndLocation _index _index_2 (Transformation|GetWorldLocation (Variables|Default|GetVolumeBox)) _returnvalue_10 _returnvalue_12 (Components|Box|GetScaledBoxExtent (Variables|Default|GetVolumeBox)))))
        ;;[1 1 1] Safety
        (if (not (Utilities|Array|IsEmpty _columnhitlocation))
          ;;[0.269 1 0.4025] Set First Row Point Location
          (Variables|Grid|SetPointLocation (Utilities|Array|Get(acopy) _columnhitlocation (Utilities|Array|LastIndex _columnhitlocation)))
          ;;[1 1 1] Height Loop
          (for _index_3 (range 0 (- _returnvalue_11 1)) :!label _label
            ;;[0.02628 0.5555 1 1 40] Sphere Collision Check
            (bind _returnvalue_13 (Collision|SphereOverlapActors (Math|Vector|MakeVector (.X (Math|Vector|BreakVector (Variables|Grid|GetPointLocation))) (.Y (Math|Vector|BreakVector (Variables|Grid|GetPointLocation))) (+ (select (not (Variables|Grid|GetbFloorTrace)) (CallFunction|CenteredGridPosition _index_3 _returnvalue_11) (- (+ (* _index_3 (Variables|Grid|GetGridSpacing)) (.Z (Math|Vector|BreakVector (Variables|Grid|GetPointLocation)))) (.z (.Min (Components|StaticMesh|GetLocalBounds (Variables|Default|GetInstancedStaticMesh)))))) (Variables|Grid|GetGridGroundOffset))) (Variables|Grid|GetOverlapRadius) (Variables|Collision|GetObjectTypes) "/Script/Engine.StaticMeshActor"))
            (if (not _returnvalue_13)
              (if (and (<= (.Z (Math|Vector|BreakVector (Math|Vector|MakeVector (.X (Math|Vector|BreakVector (Variables|Grid|GetPointLocation))) (.Y (Math|Vector|BreakVector (Variables|Grid|GetPointLocation))) (+ (select (not (Variables|Grid|GetbFloorTrace)) (CallFunction|CenteredGridPosition _index_3 _returnvalue_11) (- (+ (* _index_3 (Variables|Grid|GetGridSpacing)) (.Z (Math|Vector|BreakVector (Variables|Grid|GetPointLocation)))) (.z (.Min (Components|StaticMesh|GetLocalBounds (Variables|Default|GetInstancedStaticMesh)))))) (Variables|Grid|GetGridGroundOffset))))) (Variables|Grid|GetVolumeTopZ)) (>= (.Z (Math|Vector|BreakVector (Math|Vector|MakeVector (.X (Math|Vector|BreakVector (Variables|Grid|GetPointLocation))) (.Y (Math|Vector|BreakVector (Variables|Grid|GetPointLocation))) (+ (select (not (Variables|Grid|GetbFloorTrace)) (CallFunction|CenteredGridPosition _index_3 _returnvalue_11) (- (+ (* _index_3 (Variables|Grid|GetGridSpacing)) (.Z (Math|Vector|BreakVector (Variables|Grid|GetPointLocation)))) (.z (.Min (Components|StaticMesh|GetLocalBounds (Variables|Default|GetInstancedStaticMesh)))))) (Variables|Grid|GetGridGroundOffset))))) (Variables|Grid|GetVolumeBottomZ)))
                (Components|InstancedStaticMesh|AddInstance (Variables|Default|GetInstancedStaticMesh) (Math|Transform|MakeTransform (Math|Vector|MakeVector (.X (Math|Vector|BreakVector (Variables|Grid|GetPointLocation))) (.Y (Math|Vector|BreakVector (Variables|Grid|GetPointLocation))) (+ (select (not (Variables|Grid|GetbFloorTrace)) (CallFunction|CenteredGridPosition _index_3 _returnvalue_11) (- (+ (* _index_3 (Variables|Grid|GetGridSpacing)) (.Z (Math|Vector|BreakVector (Variables|Grid|GetPointLocation)))) (.z (.Min (Components|StaticMesh|GetLocalBounds (Variables|Default|GetInstancedStaticMesh)))))) (Variables|Grid|GetGridGroundOffset))) "0, 0, 0" (Math|Conversions|ToVector(Float) (Variables|Grid|GetPreviewMeshScale))) true)
                (Utilities|Array|Add (Variables|Default|GetSavedInstanceLocations) (Math|Vector|MakeVector (.X (Math|Vector|BreakVector (Variables|Grid|GetPointLocation))) (.Y (Math|Vector|BreakVector (Variables|Grid|GetPointLocation))) (+ (select (not (Variables|Grid|GetbFloorTrace)) (CallFunction|CenteredGridPosition _index_3 _returnvalue_11) (- (+ (* _index_3 (Variables|Grid|GetGridSpacing)) (.Z (Math|Vector|BreakVector (Variables|Grid|GetPointLocation)))) (.z (.Min (Components|StaticMesh|GetLocalBounds (Variables|Default|GetInstancedStaticMesh)))))) (Variables|Grid|GetGridGroundOffset))))))))
        (else
          (Variables|Grid|SetPointLocation (.TraceEnd (CallFunction|TraceStartEndLocation _index _index_2 (Transformation|GetWorldLocation (Variables|Default|GetVolumeBox)) _returnvalue_10 _returnvalue_12 (Components|Box|GetScaledBoxExtent (Variables|Default|GetVolumeBox)))))
          (goto _label)))))
  ;;[0.177 1 0 1 34] Generate Camera Locations
  (CallFunction|GenerateCameraLocations)
  ;;[0.177 1 0 1 34] Call Grid Updated
  (Default|CallGridUpdated))

(fn ConstructionScript
  (CallFunction|UpdateGrid))

(fn AddPositionJitter
  (params (InVec :type Vector))
  (bind (_x _y _z) (Math|Vector|BreakVector InVec))
  (bind _minmaxjitter (Variables|Grid|GetMinMaxJitter))
  (bind (_x_2 _y_2) (Math|Vector2D|BreakVector2D _minmaxjitter))
  (bind _returnvalue (Math|Float|Truncate _x_2))
  (bind _returnvalue_2 (Math|Float|Truncate _y_2))
  (bind _returnvalue_3 (Math|Random|RandomIntegerinRange _returnvalue _returnvalue_2))
  (bind _returnvalue_4 (/ _returnvalue_3 2))
  (bind _returnvalue_5 (Math|Conversions|ToFloat(Integer) _returnvalue_4))
  (return (Math|Vector|MakeVector (+ _x _returnvalue_3) (+ _y _returnvalue_3) (+ _z _returnvalue_4)) (Math|Rotator|MakeRotator _returnvalue_5 _returnvalue_5 _returnvalue_5)))

(fn GenerateCameraLocations
  (bind _baddjitter (Variables|Grid|GetbAddJitter))
  (bind _previewmeshselection (Variables|Grid|GetPreviewMeshSelection))
  (bind _returnvalue (== _previewmeshselection 2))
  (for _index (range 0 (- (Components|InstancedStaticMesh|GetInstanceCount (Variables|Default|GetInstancedStaticMesh)) 1))
    ;[1 0.1978 0.2078] True = 12 Perspectives, False = 4
    (if (== (Variables|Grid|GetPreviewMeshSelection) 2)
      (for _index_2 (range 0 2)
        (for _index_3 (range 0 3)
          (bind _output_get (Variables|Grid|SetAddedRotation (+ (Variables|Grid|GetAddedRotation) 9e+01)))
          (Utilities|Array|Add (Variables|Grid|GetSavedTransforms) (Math|Transform|MakeTransform (Math|Vector|SelectVector (.Location (CallFunction|AddPositionJitter (.location (.OutInstanceTransform (Components|InstancedStaticMesh|GetInstanceTransform (Variables|Default|GetInstancedStaticMesh) _index true))))) (.location (.OutInstanceTransform (Components|InstancedStaticMesh|GetInstanceTransform (Variables|Default|GetInstancedStaticMesh) _index true))) _baddjitter) (Math|Rotator|SelectRotator (Math|Rotator|CombineRotators (Math|Rotator|MakeRotator 0.0 (select _returnvalue (Utilities|Select :Index _index_2 :Option%200 -45.0 :Option%201 0.0 :Option%202 45.0) 0.0) (+ _output_get (select _returnvalue (Utilities|Select :Index _index_2 :Option%200 45.0 :Option%201 0.0 :Option%202 45.0) 0.0))) (.Rotation (CallFunction|AddPositionJitter (.location (.OutInstanceTransform (Components|InstancedStaticMesh|GetInstanceTransform (Variables|Default|GetInstancedStaticMesh) _index true)))))) (Math|Rotator|MakeRotator 0.0 (select _returnvalue (Utilities|Select :Index _index_2 :Option%200 -45.0 :Option%201 0.0 :Option%202 45.0) 0.0) (+ _output_get (select _returnvalue (Utilities|Select :Index _index_2 :Option%200 45.0 :Option%201 0.0 :Option%202 45.0) 0.0))) _baddjitter))))
        ;[1 0.1978 0.2078] False = 4 Perspectives, False = 6
        (if (== (Variables|Grid|GetPreviewMeshSelection) 1)
          (for _index_4 (range 0 1)
            (Utilities|Array|Add (Variables|Grid|GetSavedTransforms) (Math|Transform|MakeTransform (Math|Vector|SelectVector (.Location (CallFunction|AddPositionJitter (.location (.OutInstanceTransform (Components|InstancedStaticMesh|GetInstanceTransform (Variables|Default|GetInstancedStaticMesh) _index true))))) (.location (.OutInstanceTransform (Components|InstancedStaticMesh|GetInstanceTransform (Variables|Default|GetInstancedStaticMesh) _index true))) _baddjitter) (Math|Rotator|SelectRotator (Math|Rotator|CombineRotators (Math|Rotator|MakeRotator 0.0 (Utilities|Select :Index _index_4 :Option%200 -9e+01 :Option%201 9e+01) 0.0) (.Rotation (CallFunction|AddPositionJitter (.location (.OutInstanceTransform (Components|InstancedStaticMesh|GetInstanceTransform (Variables|Default|GetInstancedStaticMesh) _index true)))))) (Math|Rotator|MakeRotator 0.0 (Utilities|Select :Index _index_4 :Option%200 -9e+01 :Option%201 9e+01) 0.0) _baddjitter))))))
      (else
        (for _index_5 (range 0 3)
          (bind _output_get_2 (Variables|Grid|SetAddedRotation (+ (Variables|Grid|GetAddedRotation) 9e+01)))
          (Utilities|Array|Add (Variables|Grid|GetSavedTransforms) (Math|Transform|MakeTransform (Math|Vector|SelectVector (.Location (CallFunction|AddPositionJitter (.location (.OutInstanceTransform (Components|InstancedStaticMesh|GetInstanceTransform (Variables|Default|GetInstancedStaticMesh) _index true))))) (.location (.OutInstanceTransform (Components|InstancedStaticMesh|GetInstanceTransform (Variables|Default|GetInstancedStaticMesh) _index true))) _baddjitter) (Math|Rotator|SelectRotator (Math|Rotator|CombineRotators (Math|Rotator|MakeRotator 0.0 (select _returnvalue (Utilities|Select :Index _index_2 :Option%200 -45.0 :Option%201 0.0 :Option%202 45.0) 0.0) (+ _output_get_2 (select _returnvalue (Utilities|Select :Index _index_2 :Option%200 45.0 :Option%201 0.0 :Option%202 45.0) 0.0))) (.Rotation (CallFunction|AddPositionJitter (.location (.OutInstanceTransform (Components|InstancedStaticMesh|GetInstanceTransform (Variables|Default|GetInstancedStaticMesh) _index true)))))) (Math|Rotator|MakeRotator 0.0 (select _returnvalue (Utilities|Select :Index _index_2 :Option%200 -45.0 :Option%201 0.0 :Option%202 45.0) 0.0) (+ _output_get_2 (select _returnvalue (Utilities|Select :Index _index_2 :Option%200 45.0 :Option%201 0.0 :Option%202 45.0) 0.0))) _baddjitter))))
        (if (== (Variables|Grid|GetPreviewMeshSelection) 1)
          (for _index_6 (range 0 1)
            (Utilities|Array|Add (Variables|Grid|GetSavedTransforms) (Math|Transform|MakeTransform (Math|Vector|SelectVector (.Location (CallFunction|AddPositionJitter (.location (.OutInstanceTransform (Components|InstancedStaticMesh|GetInstanceTransform (Variables|Default|GetInstancedStaticMesh) _index true))))) (.location (.OutInstanceTransform (Components|InstancedStaticMesh|GetInstanceTransform (Variables|Default|GetInstancedStaticMesh) _index true))) _baddjitter) (Math|Rotator|SelectRotator (Math|Rotator|CombineRotators (Math|Rotator|MakeRotator 0.0 (Utilities|Select :Index _index_6 :Option%200 -9e+01 :Option%201 9e+01) 0.0) (.Rotation (CallFunction|AddPositionJitter (.location (.OutInstanceTransform (Components|InstancedStaticMesh|GetInstanceTransform (Variables|Default|GetInstancedStaticMesh) _index true)))))) (Math|Rotator|MakeRotator 0.0 (Utilities|Select :Index _index_6 :Option%200 -9e+01 :Option%201 9e+01) 0.0) _baddjitter)))))))))

(fn TraceStartEndLocation
  (params (X_LoopIndex :type Integer) (Y_LoopIndex :type Integer) (WorldLocation :type Vector) (XCount :type Integer) (YCount :type Integer) (BoxExtent :type Vector))
  (bind (_x _y) (Math|Vector|BreakVector BoxExtent))
  (bind _returnvalue (- WorldLocation BoxExtent))
  (bind _gridspacing (Variables|Grid|GetGridSpacing))
  (bind _gridspacing_2 (Variables|Grid|GetGridSpacing))
  (bind _gridspacing_3 (Variables|Grid|GetGridSpacing))
  (bind _returnvalue_2 (/ _gridspacing 2.0))
  (Variables|Grid|SetXTrace (+ (+ (+ (.x _returnvalue) (/ (- (* _x 2.0) (* XCount _gridspacing_3)) 2.0)) (* X_LoopIndex _gridspacing_2)) _returnvalue_2))
  (Variables|Grid|SetYTrace (+ (+ (+ (.y _returnvalue) (/ (- (* _y 2.0) (* YCount _gridspacing_3)) 2.0)) (* Y_LoopIndex _gridspacing_2)) _returnvalue_2))
  (return (Math|Vector|MakeVector (Variables|Grid|GetXTrace) (Variables|Grid|GetYTrace) (Variables|Grid|GetVolumeTopZ)) (Math|Vector|MakeVector (Variables|Grid|GetXTrace) (Variables|Grid|GetYTrace) (Variables|Grid|GetVolumeBottomZ))))

(fn FloorTrace
  (params (StartTrace :type Vector) (EndTrace :type Vector))
  ;[0 1 0.6669] Clear all Hits and Locations
  (Variables|Collision|SetbHasReachedBottom true)
  (Utilities|Array|Clear (Variables|Collision|GetActorsToIgnore))
  (Utilities|Array|Clear (Variables|Collision|GetColumnHitLocation))
  (while (Variables|Collision|GetbHasReachedBottom)
    (bind (_outhit _returnvalue) (Collision|LineTraceByChannel StartTrace EndTrace "TraceTypeQuery1" true (Variables|Collision|GetActorsToIgnore) (Variables|Debug|GetDebug)))
    ;[0.02628 0.5555 1] Finish Loop when Bottom Layer was hit
    (if _returnvalue
      ;[0 1 0.6669] Add Hits and Locations
      (Utilities|Array|Add (Variables|Collision|GetColumnHitLocation) (.location _outhit))
      (Utilities|Array|Add (Variables|Collision|GetActorsToIgnore) (.hitactor _outhit))
      (else
        (Variables|Collision|SetbHasReachedBottom false))))
  (return))

(fn CenteredGridPosition
  (params (Z_LoopIndex :type Integer) (ZCount :type Integer))
  (bind _volumebox (Variables|Default|GetVolumeBox))
  (bind _returnvalue (Components|Box|GetScaledBoxExtent _volumebox))
  (return (+ (+ (+ (.z (- (Transformation|GetWorldLocation (Variables|Default|GetVolumeBox)) _returnvalue)) (/ (- (* (.Z (Math|Vector|BreakVector _returnvalue)) 2.0) (* ZCount (Variables|Grid|GetGridSpacing))) 2.0)) (* Z_LoopIndex (Variables|Grid|GetGridSpacing))) (/ (Variables|Grid|GetGridSpacing) 2.0))))

(fn ResizePointCloudBox
  (Components|Box|SetBoxExtent (Variables|Default|GetPointCloudBox) (+ (Components|Box|GetUnscaledBoxExtent (Variables|Default|GetVolumeBox)) (/ (Variables|Grid|GetPointCloudBoxMargin) (Transformation|GetActorScale3D))) true))

(fn UpdateInstanceSize
  (for _array_element (Variables|Default|GetSavedInstanceLocations)
    (Utilities|Array|Add (LocalVariables|GetInstanceTransforms) (Math|Transform|MakeTransform _array_element "0, 0, 0" (Math|Conversions|ToVector(Float) (Variables|Grid|GetPreviewMeshScale)))))
  (Class|InstancedStaticMeshComponent|BatchUpdateInstancesTransforms (Variables|Default|GetInstancedStaticMesh) 0 (LocalVariables|GetInstanceTransforms) true true false))